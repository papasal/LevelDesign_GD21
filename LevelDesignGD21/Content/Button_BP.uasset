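; Interactive push button that toggles an activated state and signals it through CallMovePlatform, apparently to drive a moving platform.
; Entering its Box as BP_FirstPersonCharacter shows a Tutorial widget and binds MovePlatform to the character's OnPush dispatcher.
; Each push flips IsActivated, recolors two referenced lights green or red, and passes the new state on.
; Leaving the Box unbinds the handler and removes all widgets, not just the tutorial.
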(event OnComponentBeginOverlap(Box)
  (params (OverlappedComponent :type Primitive%20Component%20Object%20Reference) (OtherActor :type Actor%20Object%20Reference) (OtherComp :type Primitive%20Component%20Object%20Reference) (OtherBodyIndex :type Integer) (bFromSweep :type Boolean) (SweepResult :type Hit%20Result%20Structure%20%28by%20ref%29))
  (bind _asbp_first_person_character (Utilities|Casting|CastToBP_FirstPersonCharacter OtherActor))
  (bind _returnvalue (UserInterface|CreateWidget "/Game/Tutorial.Tutorial_C"))
  (bind _output_get (Variables|Default|SetNewVar_2 _returnvalue))
  (UserInterface|Viewport|AddtoViewport _output_get 0)
  (EventDispatchers|BindEventtoOnPush _asbp_first_person_character (delegate Custom|MovePlatform)))

(event OnComponentEndOverlap(Box)
  (params (OverlappedComponent :type Primitive%20Component%20Object%20Reference) (OtherActor :type Actor%20Object%20Reference) (OtherComp :type Primitive%20Component%20Object%20Reference) (OtherBodyIndex :type Integer))
  (bind _asbp_first_person_character (Utilities|Casting|CastToBP_FirstPersonCharacter OtherActor))
  (Viewport|RemoveAllWidgets)
  (EventDispatchers|UnbindEventfromOnPush _asbp_first_person_character (delegate Custom|MovePlatform)))

(event Custom|MovePlatform
  (params (Push :type Boolean))
  (if Push
    (if (Variables|Default|GetIsActivated)
      (Variables|Default|SetIsActivated false)
      (Rendering|Components|Light|SetLightColor (Variables|/Script/Engine.Light|GetLightComponent (Variables|Default|GetLight)) "(R=0.616319,G=0.053928,B=0.029398,A=1.000000)" true)
      (Rendering|Components|Light|SetLightColor (Variables|/Script/Engine.Light|GetLightComponent (Variables|Default|GetLight%202)) "(R=0.616319,G=0.053928,B=0.029398,A=1.000000)" true)
      (else
        (Variables|Default|SetIsActivated true)
        (Rendering|Components|Light|SetLightColor (Variables|/Script/Engine.Light|GetLightComponent (Variables|Default|GetLight)) "(R=0.179637,G=0.781250,B=0.123439,A=1.000000)" true)
        (Rendering|Components|Light|SetLightColor (Variables|/Script/Engine.Light|GetLightComponent (Variables|Default|GetLight%202)) "(R=0.179637,G=0.781250,B=0.123439,A=1.000000)" true)))
    (Default|CallMovePlatform (Variables|Default|GetIsActivated))))

(event EventBeginPlay
  (Input|EnableInput (Game|GetPlayerController 0)))

(fn ConstructionScript)